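; Player spawn point for local multiplayer that places one ThirdPersonCharacter at its own transform on BeginPlay.
; It decrements PlayerId, then either reuses the first player's existing pawn or creates a new local player with a pawn.
; The character gets a team from PlayerId parity, updates its team color and moves to the spawner.
; An unconnected chain holds an alternative manual spawn-and-possess approach that never runs.
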(event EventBeginPlay
  (bind _returnvalue (Game|Player|GetPlayerPawn 0))
  (bind _result (Math|Integer|DecrementInt (Variables|Default|GetplayerId))
    (:%20%20
      (if (== _result 0)
        (bind _asthird_person_character (Utilities|Casting|CastToThirdPersonCharacter _returnvalue))
        (Variables|/Game/Blueprints/ThirdPersonCharacter.ThirdPersonCharacter_C|Setteam _asthird_person_character (Math|Integer|%(Integer) (Variables|Default|GetplayerId) 2))
        (Default|SetTeamColor _asthird_person_character)
        (Transformation|SetActorTransform _returnvalue (Transformation|GetActorTransform))
        (else
          (bind _returnvalue_2 (Class|GameplayStatics|CreatePlayer -1))
          (bind _asthird_person_character_2 (Utilities|Casting|CastToThirdPersonCharacter (Pawn|GetControlledPawn _returnvalue_2)))
          (Variables|/Game/Blueprints/ThirdPersonCharacter.ThirdPersonCharacter_C|Setteam _asthird_person_character_2 (Math|Integer|%(Integer) (Variables|Default|GetplayerId) 2))
          (Default|SetTeamColor _asthird_person_character_2)
          (Transformation|SetActorTransform (Pawn|GetControlledPawn _returnvalue_2) (Transformation|GetActorTransform)))))))

(fn ConstructionScript)